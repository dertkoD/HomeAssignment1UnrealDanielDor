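; Ammo pickup actor that adds reserve ammo to the character who interacts with it.
; On Interact, it asks that character for a weapon of its configured ammo weapon type.
; If one is found, it adds its ammo amount to the reserve for that weapon's type and destroys itself; otherwise it stays in the world.
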(event `/Game/_Main/Interfaces/BPI_Interact.Interact`
  (params (`Character Picking Up` :type "/Game/FirstPerson/Blueprints/BP_FirstPersonCharacter Object Reference"))
  (bind (_current_weapon_of_type _has_weapon_of_type) (`/Game/FirstPerson/Blueprints/BP_FirstPersonCharacter.Get Weapon Of Type` `Character Picking Up` (`self.AmmoWeaponType`)))
  (if _has_weapon_of_type
    (`/Game/FirstPerson/Blueprints/BP_FirstPersonCharacter.Add Ammo To Reserve` `Character Picking Up` (`/Game/_Main/Weapons/BP_Weapon_Master.Weapon Type` _current_weapon_of_type) (`self.AmmoAmount`))
    (`self.K2_DestroyActor`)))

(fn `UserConstructionScript`
  (`parent.UserConstructionScript`))