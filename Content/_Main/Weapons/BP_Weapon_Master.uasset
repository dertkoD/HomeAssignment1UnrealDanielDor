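; BP_Weapon_Master is a weapon Blueprint, apparently a base for guns, that handles semi-auto and full-auto firing with magazine ammo.
; StartFire fires once, and full-auto also starts a looping timer at the FireRate interval, which StopFire clears.
; FireOnce spends a round, plays the firing animation and spawns a projectile at the barrel socket.
; An empty magazine stops firing and plays a sound at world origin; AddAmmoToMag refills within MagSize.
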(event `Start Fire`
  (set `self.Is Firing` true)
  (switch `/Game/_Main/Weapons/Enum_FireMode` (`self.Fire Mode`)
    (:`NewEnumerator0`
      (`self.Fire Once`))
    (:`NewEnumerator1`
      (`KismetSystemLibrary.K2_ClearAndInvalidateTimerHandle` (`self.Fire Timer Handle`))
      (`self.Fire Once`)
      (bind _returnvalue (`KismetSystemLibrary.K2_SetTimerDelegate` (`|CreateDelegate` :!event `Fire Once`) (/ 1.0 (`KismetMathLibrary.FMax` (`self.Fire Rate`) 0.01)) true))
      (set `self.Fire Timer Handle` _returnvalue))))

(event `Stop Fire`
  (set `self.Is Firing` false)
  (`KismetSystemLibrary.K2_ClearAndInvalidateTimerHandle` (`self.Fire Timer Handle`)))

(event `Fire Once`
  (bind (_returnvalue_location _returnvalue_rotation) (`KismetMathLibrary.BreakTransform` (`self.GetSocketTransform` "barrel")))
  (bind _ammo_in_mag (`self.Ammo In Mag`))
  (if (> _ammo_in_mag 0)
    (set `self.Ammo In Mag` (- _ammo_in_mag 1))
    (`self.PlayAnimation` (`self.Firing Animation`))
    (`|SpawnActorFromClass` "/Game/_Main/Projectiles/BP_Projectiles_Master.BP_Projectiles_Master_C" (`KismetMathLibrary.MakeTransform` _returnvalue_location _returnvalue_rotation) "Undefined" "MultiplyWithRoot" null null)
    (else
      (`self.Stop Fire`)
      (`GameplayStatics.PlaySoundAtLocation` "/Game/MilitaryWeapDark/Sound/Pistol/Pistol_MagEject_Cue.Pistol_MagEject_Cue" (0.0 0.0 0.0) (struct) 1.0 1.0 0.0 null null null null))))

(fn `AddAmmoToMag`
  (params (Amount :type Integer))
  (set `self.Ammo In Mag` (`KismetMathLibrary.Clamp` (+ Amount (`self.Ammo In Mag`)) 0 (`self.MagSize`))))