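; Zombie enemy that patrols waypoints, chases the player on sight and triggers game over when its kill capsule touches them.
; A detection sphere starts timed line-of-sight traces, driving a patrol, alert and chase state machine through timers and AIMoveTo, with an alert delay facing the player before chasing.
; Damage updates the player's enemy HP UI; death ragdolls the mesh and unregisters it from the main widget, where it registered on spawn.
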(event `self.ReceiveBeginPlay`
  (`self.StartPatrol`)
  (bind _returnvalue (`KismetSystemLibrary.K2_SetTimerDelegate` (delegate `Try Register Enemy`) 0.1 true))
  (set `self.RegisterTimerHandle` _returnvalue))

(event `Try Register Enemy`
  (bind _asbp_first_person_character (cast `/Game/FirstPerson/Blueprints/BP_FirstPersonCharacter` (`GameplayStatics.GetPlayerCharacter` 0)))
  (bind _mainwidgetref (`/Game/FirstPerson/Blueprints/BP_FirstPersonCharacter.MainWidgetRef` _asbp_first_person_character))
  (`/Engine/EditorBlueprintResources/StandardMacros.IsValid` _mainwidgetref
    (:`Is Valid`
      (`/Game/_Main/Widget/UI_Main.RegisterEnemy` _mainwidgetref 1)
      (`KismetSystemLibrary.K2_ClearAndInvalidateTimerHandle` (`self.RegisterTimerHandle`))
      (`PrimitiveComponent.SetCollisionEnabled` (`self.SphereDetection`) "QueryAndPhysics")
      (`PrimitiveComponent.SetCollisionEnabled` (`self.CapsuleKill`) "QueryAndPhysics"))))

(event `StartPatrol`
  (set `self.State` "NewEnumerator0")
  (set `CharacterMovementComponent.MaxWalkSpeed` (`self.Speed Patrol`) (`self.CharacterMovement`))
  (`self.MoveToNextPatrolPoint`))

(event `MoveToNextPatrolPoint`
  (bind _patrolpoints (`self.PatrolPoints`))
  (bind _patrolindex (`self.PatrolIndex`))
  (bind _returnvalue (`KismetArrayLibrary.Array_Length` _patrolpoints))
  (if (> _returnvalue 0)
    (`|AIMoveTo` self (0.0 0.0 0.0) (`|GetArrayItem` _patrolpoints _patrolindex) 80.0
      (:`OnSuccess`
        (bind _result (`/Engine/EditorBlueprintResources/StandardMacros.IncrementInt` _patrolindex)
          (:`  `
            (set `self.PatrolIndex` (mod _result _returnvalue))
            (`self.MoveToNextPatrolPoint`)))))))

(event `self.ReceiveAnyDamage`
  (params (Damage :type "Float (single-precision)") (DamageType :type "DamageType Object Reference") (InstigatedBy :type "Controller Object Reference") (DamageCauser :type "Actor Object Reference"))
  (if (> (`self.Health`) 0.0)
    (bind _output_get (set `self.Health` (`KismetMathLibrary.FClamp` (- (`self.Health`) Damage) 0.0 (`self.Max Health`))))
    (bind _asbp_first_person_character (cast `/Game/FirstPerson/Blueprints/BP_FirstPersonCharacter` (`GameplayStatics.GetPlayerCharacter` 0)))
    (`/Game/FirstPerson/Blueprints/BP_FirstPersonCharacter.ShowEnemyHP_UI` _asbp_first_person_character _output_get)
    (if (<= (`self.Health`) 0.0)
      (`self.Death`))))

(event `Death`
  (bind _mesh (`self.Mesh`))
  (if (not (`self.Is Dead`))
    (set `self.Is Dead` true)
    (set `self.State` "NewEnumerator0")
    (`self.Cleat All Timers`)
    (`PrimitiveComponent.SetCollisionEnabled` _mesh "QueryAndPhysics")
    (`PrimitiveComponent.SetSimulatePhysics` _mesh true)
    (`SkeletalMeshComponent.SetPhysicsBlendWeight` _mesh 1.0)
    (`PrimitiveComponent.SetCollisionEnabled` (`self.CapsuleComponent`) "NoCollision")
    (bind _asbp_first_person_character (cast `/Game/FirstPerson/Blueprints/BP_FirstPersonCharacter` (`GameplayStatics.GetPlayerCharacter` 0)))
    (`/Game/_Main/Widget/UI_Main.UnregisterEnemy` (`/Game/FirstPerson/Blueprints/BP_FirstPersonCharacter.MainWidgetRef` _asbp_first_person_character) 1)))

(event `self.CapsuleKill.OnComponentBeginOverlap`
  (params (OverlappedComponent :type "PrimitiveComponent Object Reference") (OtherActor :type "Actor Object Reference") (OtherComp :type "PrimitiveComponent Object Reference") (OtherBodyIndex :type Integer) (bFromSweep :type Boolean) (SweepResult :type "HitResult Structure (by ref)"))
  (bind _asbp_first_person_character (cast `/Game/FirstPerson/Blueprints/BP_FirstPersonCharacter` OtherActor))
  (`/Game/FirstPerson/Blueprints/BP_FirstPersonCharacter.Game Over` _asbp_first_person_character)
  (set `self.bIgnorePlayer` true)
  (set `self.bPlayerInRange` false)
  (set `self.PlayerRef` null)
  (`self.Cleat All Timers`)
  (`PrimitiveComponent.SetCollisionEnabled` (`self.SphereDetection`) "NoCollision")
  (`PrimitiveComponent.SetCollisionEnabled` (`self.CapsuleKill`) "NoCollision")
  (`self.StopChaseAndReturnToPatrol`))

(event `self.SphereDetection.OnComponentBeginOverlap`
  (params (OverlappedComponent :type "PrimitiveComponent Object Reference") (OtherActor :type "Actor Object Reference") (OtherComp :type "PrimitiveComponent Object Reference") (OtherBodyIndex :type Integer) (bFromSweep :type Boolean) (SweepResult :type "HitResult Structure (by ref)"))
  (bind _asbp_first_person_character (cast `/Game/FirstPerson/Blueprints/BP_FirstPersonCharacter` OtherActor))
  (set `self.PlayerRef` _asbp_first_person_character)
  (set `self.bPlayerInRange` true)
  (`KismetSystemLibrary.K2_ClearAndInvalidateTimerHandle` (`self.LostTimerHandle`))
  (`KismetSystemLibrary.K2_ClearAndInvalidateTimerHandle` (`self.SightTimerHandle`))
  (bind _returnvalue (`KismetSystemLibrary.K2_SetTimerDelegate` (delegate `UpdateSight`) (`self.SightCheckRate`) true))
  (set `self.SightTimerHandle` _returnvalue)
  (`self.TryStartChase`))

(event `UpdateSight`
  (if (`self.bPlayerInRange`)
    (`/Engine/EditorBlueprintResources/StandardMacros.IsValid` (`self.PlayerRef`)
      (:`Is Valid`
        (bind _haslostoplayer (`self.HasLOSToPlayer`))
        (if _haslostoplayer
          (`self.TryStartChase`)
          (elif (`|EnumEquality` (`self.State`) "NewEnumerator2")
            (`self.CancelAlertReturnToPatrol`)))))))

(event `self.SphereDetection.OnComponentEndOverlap`
  (params (OverlappedComponent :type "PrimitiveComponent Object Reference") (OtherActor :type "Actor Object Reference") (OtherComp :type "PrimitiveComponent Object Reference") (OtherBodyIndex :type Integer))
  (cast `/Game/FirstPerson/Blueprints/BP_FirstPersonCharacter` OtherActor)
  (if (== OtherActor (`self.PlayerRef`))
    (if (`|EnumEquality` (`self.State`) "NewEnumerator2")
      (`self.CancelAlertReturnToPatrol`)
      (else
        (set `self.bPlayerInRange` false)
        (`KismetSystemLibrary.K2_ClearAndInvalidateTimerHandle` (`self.SightTimerHandle`))
        (bind _returnvalue (`KismetSystemLibrary.K2_SetTimerDelegate` (`|CreateDelegate` :!event `OnLosePlayerTimeout`) (`self.LoseDelay`)))
        (set `self.LostTimerHandle` _returnvalue)))))

(event `Start Chase`
  (set `self.State` "NewEnumerator1")
  (`KismetSystemLibrary.K2_ClearAndInvalidateTimerHandle` (`self.AlertTimerHandle`))
  (`KismetSystemLibrary.K2_ClearAndInvalidateTimerHandle` (`self.AlertLookTimerHandle`))
  (set `CharacterMovementComponent.MaxWalkSpeed` (`self.Speed Chase`) (`self.CharacterMovement`))
  (`KismetSystemLibrary.K2_ClearAndInvalidateTimerHandle` (`self.ChaseTimerHandle`))
  (`self.UpdateChase`)
  (bind _returnvalue (`KismetSystemLibrary.K2_SetTimerDelegate` (delegate `UpdateChase`) (`self.ChaseUpdateRate`)))
  (set `self.ChaseTimerHandle` _returnvalue))

(event `OnLosePlayerTimeout`
  (bind _playerref (`self.PlayerRef`))
  (if (`|EnumEquality` (`self.State`) "NewEnumerator1")
    (`/Engine/EditorBlueprintResources/StandardMacros.IsValid` _playerref
      (:`Is Valid`
        (if (not (`PrimitiveComponent.IsOverlappingActor` (`self.SphereDetection`) _playerref))
          (`self.StopChaseAndReturnToPatrol`))))))

(event `UpdateChase`
  (bind _playerref (`self.PlayerRef`))
  (if (`|EnumEquality` (`self.State`) "NewEnumerator1")
    (`/Engine/EditorBlueprintResources/StandardMacros.IsValid` _playerref
      (:`Is Valid`
        (bind _haslostoplayer (`self.HasLOSToPlayer`))
        (if _haslostoplayer
          (`|AIMoveTo` self (0.0 0.0 0.0) _playerref (`self.KillDistance`) true
            (:`OnSuccess`
              (`KismetSystemLibrary.K2_ClearAndInvalidateTimerHandle` (`self.ChaseTimerHandle`))))))
      (:`Is Not Valid`
        (`self.StartPatrol`)))))

(event `StopChaseAndReturnToPatrol`
  (set `self.State` "NewEnumerator0")
  (`KismetSystemLibrary.K2_ClearAndInvalidateTimerHandle` (`self.ChaseTimerHandle`))
  (`self.StartPatrol`))

(event `TryStartChase`
  (if (`self.bPlayerInRange`)
    (bind _haslostoplayer (`self.HasLOSToPlayer`))
    (if _haslostoplayer
      (if (`|EnumEquality` (`self.State`) "NewEnumerator0")
        (`self.StartAlert`)))))

(event `StartAlert`
  (set `self.State` "NewEnumerator2")
  (`MovementComponent.StopMovementImmediately` (`self.CharacterMovement`))
  (`KismetSystemLibrary.K2_ClearAndInvalidateTimerHandle` (`self.AlertTimerHandle`))
  (`KismetSystemLibrary.K2_ClearAndInvalidateTimerHandle` (`self.AlertLookTimerHandle`))
  (bind _returnvalue (`KismetSystemLibrary.K2_SetTimerDelegate` (delegate `UpdateAlertLook`) (`self.AlertLookRate`) true))
  (set `self.AlertLookTimerHandle` _returnvalue)
  (bind _returnvalue_2 (`KismetSystemLibrary.K2_SetTimerDelegate` (delegate `ConfirmChaseAfterAlert`) (`self.AlertDelay`)))
  (set `self.AlertTimerHandle` _returnvalue_2))

(event `ConfirmChaseAfterAlert`
  (if (`|EnumEquality` (`self.State`) "NewEnumerator2")
    (`/Engine/EditorBlueprintResources/StandardMacros.IsValid` (`self.PlayerRef`)
      (:`Is Valid`
        (bind _haslostoplayer (`self.HasLOSToPlayer`))
        (if _haslostoplayer
          (`self.Start Chase`)))
      (:`Is Not Valid`
        (`self.CancelAlertReturnToPatrol` :!label _label)))
    (else
      (goto _label))))

(event `UpdateAlertLook`
  (bind _playerref (`self.PlayerRef`))
  (if (`|EnumEquality` (`self.State`) "NewEnumerator2")
    (`/Engine/EditorBlueprintResources/StandardMacros.IsValid` _playerref
      (:`Is Valid`
        (`self.K2_SetActorRotation` (`KismetMathLibrary.FindLookAtRotation` (`self.K2_GetActorLocation`) (`self.K2_GetActorLocation` _playerref))))
      (:`Is Not Valid`
        (`self.CancelAlertReturnToPatrol` :!label _label_2)))
    (else
      (goto _label_2))))

(event `CancelAlertReturnToPatrol`
  (`KismetSystemLibrary.K2_ClearAndInvalidateTimerHandle` (`self.AlertTimerHandle`))
  (`KismetSystemLibrary.K2_ClearAndInvalidateTimerHandle` (`self.AlertLookTimerHandle`))
  (`self.StartPatrol`))

(fn `Cleat All Timers`
  (`KismetSystemLibrary.K2_ClearAndInvalidateTimerHandle` (`self.SightTimerHandle`))
  (`KismetSystemLibrary.K2_ClearAndInvalidateTimerHandle` (`self.LostTimerHandle`))
  (`KismetSystemLibrary.K2_ClearAndInvalidateTimerHandle` (`self.ChaseTimerHandle`))
  (`KismetSystemLibrary.K2_ClearAndInvalidateTimerHandle` (`self.AlertTimerHandle`)))

(fn `HasLOSToPlayer`
  (returns (HasLOSToPlayer :type Boolean))
  (bind (_outhit _returnvalue) (`KismetSystemLibrary.LineTraceSingle` :`Start` (+ (`self.K2_GetActorLocation`) (0.0 0.0 50.0)) :`End` (+ (`self.K2_GetActorLocation` (`self.PlayerRef`)) (0.0 0.0 50.0)) :`TraceChannel` "TraceTypeQuery1" :`DrawDebugType` "ForDuration" :`DrawTime` 15.0))
  (return (and _returnvalue (== (`.HitActor` (`GameplayStatics.BreakHitResult` _outhit)) (`self.PlayerRef`)))))

(fn `UserConstructionScript`)